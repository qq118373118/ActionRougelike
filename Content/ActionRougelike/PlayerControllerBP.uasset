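; Player controller Blueprint for the action roguelike that sets up the local player's HUD and provides test hotkeys.
; On begin playing state, the local controller creates the Main_HUD widget, adds it to the viewport and switches to game-only input.
; Hard-coded keys call into SGameModeBase to write the save game (L) and into SPlayerState to grant credits (1), each printing a confirmation message.
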(event EventBlueprintBeginPlayingState
  (if (Pawn|IsLocalController)
    (bind _returnvalue (UserInterface|CreateWidget "/Game/ActionRougelike/UI/Main_HUD.Main_HUD_C"))
    (UserInterface|Viewport|AddtoViewport _returnvalue 0)
    (Input|SetInputModeGameOnly self)))

(event Input|KeyboardEvents|L
  (params (Key :type Key%20Structure :default "None"))
  (:Pressed
    (bind _assgame_mode_base (Utilities|Casting|CastToSGameModeBase (Game|GetGameMode)))
    (Class|SGameModeBase|WriteSaveGame _assgame_mode_base)
    (Development|PrintString "World Saveed")))

(event Input|KeyboardEvents|1
  (params (Key :type Key%20Structure :default "None"))
  (:Pressed
    (bind _assplayer_state (Utilities|Casting|CastToSPlayerState (Variables|Default|GetPlayerState)))
    (Class|SPlayerState|AddCredits _assplayer_state 50)
    (Development|PrintString "add 50 point")))

(fn ConstructionScript)